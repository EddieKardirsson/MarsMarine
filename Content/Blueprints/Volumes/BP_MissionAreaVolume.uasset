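; BP_MissionAreaVolume is a mission boundary volume that punishes the player for deserting the play area.
; Leaving the volume flags a BP_Marine as outside the mission area and starts a KillDeserter timer, which re-entry clears.
; On expiry, KillDeserter deals fixed damage to player 0's marine, regardless of which marine started the timer.
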(event `self.ReceiveActorBeginOverlap`
  (params (OtherActor :type "Actor Object Reference"))
  (bind _asbp_marine (cast `/Game/Blueprints/Pawns/BP_Marine` OtherActor))
  (set `/Game/Blueprints/Pawns/BP_Marine.OutsideMissionArea` false _asbp_marine)
  (`KismetSystemLibrary.K2_ClearTimer` null "KillDeserter"))

(event `self.ReceiveActorEndOverlap`
  (params (OtherActor :type "Actor Object Reference"))
  (bind _asbp_marine (cast `/Game/Blueprints/Pawns/BP_Marine` OtherActor))
  (set `/Game/Blueprints/Pawns/BP_Marine.OutsideMissionArea` true _asbp_marine)
  (`KismetSystemLibrary.K2_SetTimer` null "KillDeserter" (`self.DeserterTimer`)))

(fn `KillDeserter`
  (bind _asbp_marine (cast `/Game/Blueprints/Pawns/BP_Marine` (`GameplayStatics.GetPlayerCharacter` 0)))
  (`GameplayStatics.ApplyDamage` _asbp_marine 100.0))

(fn `UserConstructionScript`)